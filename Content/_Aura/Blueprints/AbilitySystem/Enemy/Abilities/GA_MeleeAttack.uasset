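; Enemy melee attack gameplay ability that turns the avatar toward its combat target and plays a random tagged attack montage.
; The montage's tag event triggers a small sphere query at the matching combat socket, with a debug sphere drawn, damaging non-friendly live players inside.
; Any hit fires a MeleeImpact gameplay cue carrying the montage tag.
; The ability ends after that event or when the montage completes, is interrupted or is cancelled.
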(event Ability|EventActivateAbility
  (bind _returnvalue (Ability|GetAvatarActorfromActorInfo))
  (bind _returnvalue_2 (Ability|GetAvatarActorfromActorInfo))
  (Variables|Default|SetHasHitTarget false)
  (bind _returnvalue_3 (Class|EnemyInterface|GetCombatTarget(Message) _returnvalue_2))
  (Class|CombatInterface|UpdateFacingTarget(Message) _returnvalue_2 (Transformation|GetActorLocation _returnvalue_3))
  (bind _returnvalue_4 (Class|CombatInterface|GetAttackMontages(Message) _returnvalue_2))
  (Variables|Default|SetTaggedMantage (Class|AuraDamageGameplayAbility|GetRandomTaggedMontage _returnvalue_4))
  (|PlayMontageandWaitProxy "None" (.montage (Variables|Default|GetTaggedMantage)) 1.0 "None" true 1.0 0.0 false
    (:then
      (Ability|Tasks|WaitGameplayEvent (.montagetag (Variables|Default|GetTaggedMantage)) 0
        (:EventReceived
          (bind _returnvalue_5 (Class|CombatInterface|GetCombatSocketLocation(Message) _returnvalue (.sockettag (Variables|Default|GetTaggedMantage))))
          (Variables|Default|SetCombatSocketLocation _returnvalue_5)
          (bind _outoverlappingactors (Class|AuraAbilitySystemLibrary|GetLivePlayersWithinRadius self (Utilities|Array|MakeArray _returnvalue) 45.0 _returnvalue_5))
          (Rendering|Debug|DrawDebugSphere (Variables|Default|GetCombatSocketLocation) 45.0 12 "(R=1.000000,G=0.000000,B=0.000000,A=1.000000)" 5.0 2.0)
          (for _array_element _outoverlappingactors
            (if (Class|AuraAbilitySystemLibrary|IsNotFriend (Ability|GetAvatarActorfromActorInfo) _array_element)
              (Class|AuraDamageGameplayAbility|CauseDamage _array_element)
              (Variables|Default|SetHasHitTarget true)))
          (if (Variables|Default|GetHasHitTarget)
            (bind _returnvalue_6 (Class|EnemyInterface|GetCombatTarget(Message) (Ability|GetAvatarActorfromActorInfo)))
            (Class|GameplayAbility|ExecuteGameplayCuewithParams "(TagName=\"GameplayCue.MeleeImpact\")" (Ability|GameplayCue|MakeGameplayCueParameters :AggregatedSourceTags (GameplayTags|MakeGameplayTagContainerfromTag (Utilities|Struct|BreakTaggedMontage (Variables|Default|GetTaggedMantage))) :Location (Variables|Default|GetCombatSocketLocation) :EffectCauser (Ability|GetAvatarActorfromActorInfo) :SourceObject _returnvalue_6)))
          (Ability|EndAbility))))
    (:OnCompleted
      (Ability|EndAbility :!label _label))
    (:OnInterrupted
      (goto _label))
    (:OnCancelled
      (goto _label))))