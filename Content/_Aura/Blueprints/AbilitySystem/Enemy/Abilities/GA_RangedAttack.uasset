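; GA_RangedAttack is an enemy gameplay ability that performs a montage-driven projectile attack on the combat target.
; On activation it updates the avatar's facing toward the target and plays a random tagged attack montage.
; When the montage's gameplay event fires, it spawns a projectile from the tagged socket toward the target's current location, with optional pitch override.
; The ability ends when the montage completes or is interrupted.
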(event Ability|EventActivateAbility
  (bind _returnvalue (Ability|GetAvatarActorfromActorInfo))
  (bind _returnvalue_2 (Class|EnemyInterface|GetCombatTarget(Message) _returnvalue))
  (Class|CombatInterface|UpdateFacingTarget(Message) _returnvalue (Transformation|GetActorLocation _returnvalue_2))
  (bind _returnvalue_3 (Class|CombatInterface|GetAttackMontages(Message) _returnvalue))
  (Variables|Default|SetTaggedMontage (Class|AuraDamageGameplayAbility|GetRandomTaggedMontage _returnvalue_3))
  (|PlayMontageandWaitProxy "None" (.montage (Variables|Default|GetTaggedMontage)) 1.0 "None" true 1.0 0.0 false
    (:then
      (Ability|Tasks|WaitGameplayEvent (.montagetag (Variables|Default|GetTaggedMontage)) 0 true
        (:EventReceived
          (bind _returnvalue_4 (Class|EnemyInterface|GetCombatTarget(Message) (Ability|GetAvatarActorfromActorInfo)))
          (Class|AuraProjectileSpell|SpawnProjectile (Transformation|GetActorLocation _returnvalue_4) (.sockettag (Variables|Default|GetTaggedMontage)) (Variables|Default|GetOverride%20Pitch) (Variables|Default|GetPitch%20Override)))))
    (:OnCompleted
      (Ability|EndAbility :!label _label))
    (:OnInterrupted
      (goto _label))))