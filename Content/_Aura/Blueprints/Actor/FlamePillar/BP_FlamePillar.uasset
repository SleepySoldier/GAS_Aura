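; BP_FlamePillar is a flame pillar actor that makes its point light flicker like fire.
; On BeginPlay it randomly plays one of two intensity timelines, each meant to pick again when finished for a varied, endless flicker.
; Timeline updates feed ScaleFlameIntensity, which multiplies the curve value by BaseIntensity and applies it to the PointLight.
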(event Custom|ChooseTimeline
  (if (Math|Random|RandomBool)
    (Components|Timeline|PlayfromStart (Variables|Default|GetFlameTimeline))
    (else
      (Components|Timeline|PlayfromStart (Variables|Default|GetFlameIntensity_2)))))

(event EventBeginPlay
  (CallFunction|ChooseTimeline))

(fn ConstructionScript)

(fn ScaleFlameIntensity
  (params (Intensity :type Float%20%28double-precision%29))
  (Rendering|Components|Light|SetIntensity (Variables|Default|GetPointLight) (* Intensity (Variables|Default|GetBaseIntensity))))