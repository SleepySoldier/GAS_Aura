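; Base pickup actor in the potion folder that applies an instant Gameplay Ability System effect to whatever overlaps its sphere.
; On overlap it passes the actor and the instant effect class to ApplyEffectToTarget, then destroys itself unconditionally.
; A separate Blueprint version, not called by the overlap event, builds the effect spec at actor level and self-destructs only if the target has an ability system component.
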(event OnComponentBeginOverlap(Sphere)
  (params (OverlappedComponent :type Primitive%20Component%20Object%20Reference) (OtherActor :type Actor%20Object%20Reference) (OtherComp :type Primitive%20Component%20Object%20Reference) (OtherBodyIndex :type Integer) (bFromSweep :type Boolean) (SweepResult :type Hit%20Result%20Structure%20%28by%20ref%29))
  (Class|AuraEffectActor|ApplyEffecttoTarget OtherActor (Variables|Default|GetInstantGameplayEffectClass))
  (Actor|DestroyActor))

(fn ConstructionScript)

(fn ApplyEffecttoTargetBP
  (params (TargetActor :type Actor%20Object%20Reference))
  (bind _returnvalue (Ability|GetAbilitySystemComponent TargetActor))
  (Utilities|IsValid _returnvalue
    (:Is%20Valid
      (GameplayEffects|ApplyGameplayEffectSpecToSelf _returnvalue (GameplayEffects|MakeOutgoingSpec _returnvalue (Variables|Default|GetInstantGameplayEffectClass) (Variables|Default|GetActorLevel) (GameplayEffects|MakeEffectContext _returnvalue)))
      (Actor|DestroyActor))))